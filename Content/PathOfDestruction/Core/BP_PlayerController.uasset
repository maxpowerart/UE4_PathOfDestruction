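; Player controller for Path of Destruction that owns the menu widget and handles pausing.
; On BeginPlay it creates WBP_Menu, adding it to the viewport and playing its Open animation only in level "123".
; The Menu input toggles pause and cursor visibility, plays MenuOpen forward or in reverse, and disables input for a short delay before switching between game-and-UI and game-only input modes.
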(event `self.ReceiveBeginPlay`
  ;[1 1 1] Construct widget
  (bind _returnvalue (`|CreateWidget` "/Game/PathOfDestruction/UI/WBP_Menu.WBP_Menu_C" self))
  (bind _output_get (set `self.HUD` _returnvalue))
  (bind _returnvalue_2 (`GameplayStatics.GetCurrentLevelName` true))
  (if (`KismetStringLibrary.EqualEqual_StrStr` _returnvalue_2 "123")
    (`UserWidget.AddToViewport` _output_get 0)
    (`UserWidget.PlayAnimation` _output_get (`/Game/PathOfDestruction/UI/WBP_Menu.Open` _output_get) 0.0 1 "Forward" 1.0 false)))

(event `InputAction|Menu` :paused true
  (params (Key :type "Key Structure"))
  (bind _hud (`self.HUD`))
  (bind _hud_2 (`self.HUD`))
  ;[1 1 1] Menu
  (:`Pressed`
    (if (not (`GameplayStatics.IsGamePaused`))
      (`GameplayStatics.SetGamePaused` true)
      (set `self.bShowMouseCursor` true)
      (`UserWidget.PlayAnimation` (`self.HUD`) (`/Game/PathOfDestruction/UI/WBP_Menu.MenuOpen` _hud) 0.0 1 "Forward" 1.0 false)
      (`self.DisableInput` self)
      (`KismetSystemLibrary.Delay` 1.0)
      (`self.EnableInput` self)
      (`WidgetBlueprintLibrary.SetInputMode_GameAndUIEx` self _hud "DoNotLock" false)
      (else
        (`GameplayStatics.SetGamePaused` false)
        (set `self.bShowMouseCursor` false)
        (`UserWidget.PlayAnimation` _hud_2 (`/Game/PathOfDestruction/UI/WBP_Menu.MenuOpen` _hud_2) 0.0 1 "Reverse" 1.0 false)
        (`self.DisableInput` self)
        (`KismetSystemLibrary.Delay` 1.0)
        (`self.EnableInput` self)
        (`WidgetBlueprintLibrary.SetInputMode_GameOnly` self)))))

(fn `UserConstructionScript`)
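; Player controller for Path of Destruction that owns the HUD and toggles the in-game pause menu.
; On BeginPlay it creates the WBP_Hud widget and adds it to the viewport.
; The Menu input shows or hides the HUD's menu, pausing the game and toggling the mouse cursor.
; Opening switches to game-and-UI input focused on the HUD; closing does not restore game-only input.
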(event `self.ReceiveBeginPlay`
  ;[1 1 1] Construct widget
  (bind _returnvalue (`|CreateWidget` "/Game/PathOfDestruction/WBP_Hud.WBP_Hud_C" self))
  (bind _output_get (set `self.HUD` _returnvalue))
  (`UserWidget.AddToViewport` _output_get 0))

(event `InputAction|Menu` :paused true
  (params (Key :type "Key Structure"))
  (bind _menu (`/Game/PathOfDestruction/WBP_Hud.Menu` (`self.HUD`)))
  ;[1 1 1] Menu
  ;;[1 0.1366 0] Close all widgets before
  (:`Pressed`
    (if (not (`Widget.IsVisible` (`/Game/PathOfDestruction/WBP_Hud.Menu` (`self.HUD`))))
      (`GameplayStatics.SetGamePaused` true)
      (set `self.bShowMouseCursor` true)
      (`WidgetBlueprintLibrary.SetInputMode_GameAndUIEx` self (`self.HUD`) "DoNotLock" false)
      (`Widget.SetVisibility` _menu "Visible")
      (else
        (`GameplayStatics.SetGamePaused` false)
        (set `self.bShowMouseCursor` false)
        (`Widget.SetVisibility` _menu "Hidden")))))

(fn `UserConstructionScript`)
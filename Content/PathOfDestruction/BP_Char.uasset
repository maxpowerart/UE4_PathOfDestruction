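; BP_Char is a Paper2D player character that moves in the X-Z plane.
; MoveRight and MoveTop axis inputs add movement along world X and Z.
; Tick flips the sprite by rotation to match the X velocity sign and plays the movement flipbook.
; It switches to the idle flipbook only at zero velocity, so purely vertical motion keeps the current flipbook.
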(event `self.ReceiveTick`
  (params (DeltaSeconds :type "Float (single-precision)"))
  (bind _returnvalue_x (`KismetMathLibrary.BreakVector` (`self.GetVelocity`)))
  (bind _sprite (`self.Sprite`))
  (if (!= _returnvalue_x 0.0)
    (if (> _returnvalue_x 0.0)
      (`SceneComponent.K2_SetRelativeRotation` _sprite (struct :`Yaw` -180.0) false false)
      (else
        (`SceneComponent.K2_SetRelativeRotation` _sprite (struct) false false)))
    (`PaperFlipbookComponent.SetFlipbook` (`self.Sprite`) "/Game/PathOfDestruction/1_Tiles/PNG/Wraith_01/PNG_Sequences/Walking/FB_Movement.FB_Movement")
    (elif (== (`KismetMathLibrary.VSize` (`self.GetVelocity`)) 0.0)
      (`PaperFlipbookComponent.SetFlipbook` (`self.Sprite`) "/Game/PathOfDestruction/1_Tiles/PNG/Wraith_01/PNG_Sequences/Idle/FB_Idle.FB_Idle"))))

(event `InputAxis|MoveTop`
  (params (AxisValue :type "Float (single-precision)"))
  (`self.AddMovementInput` (0.0 0.0 1.0) AxisValue))

(event `InputAxis|MoveRight`
  (params (AxisValue :type "Float (single-precision)"))
  (`self.AddMovementInput` (1.0 0.0 0.0) AxisValue))

(fn `UserConstructionScript`)
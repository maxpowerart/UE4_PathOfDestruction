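; Possessable dialog scene that shows speaker, text and two clickable option widgets from a DlgContext, then returns control to BP_Char when dialog ends.
; Possession sets up cursor input and refreshes widgets; mouse or Enter picks the first option when no second exists.
; SetDisType applies handicaps, run from Tick through resettable DoOnce gates: a randomly bouncing option, or a grid of decoy buttons copying one option around the other.
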(event `Key|LeftMouseButton`
  (params (Key :type "Key Structure"))
  (:`Pressed`
    (if (and (not (`DlgContext.IsValidOptionIndex` (`self.DlgContext`) 1)) (not (`self.ChooseBuffer`))) :!label _label
      (bind _aswbp_dialog_option (cast `/Game/PathOfDestruction/UI/WBP_DialogOption` (`WidgetComponent.GetWidget` (`self.First`))))
      (`/Game/PathOfDestruction/UI/WBP_DialogOption.Clicked` _aswbp_dialog_option))))

(event `self.First.OnClicked`
  (params (TouchedComponent :type "PrimitiveComponent Object Reference") (ButtonPressed :type "Key Structure"))
  ;[1 1 1] OnButtonClick
  (bind _aswbp_dialog_option (cast `/Game/PathOfDestruction/UI/WBP_DialogOption` (`WidgetComponent.GetWidget` (`self.First`))))
  (`/Game/PathOfDestruction/UI/WBP_DialogOption.Clicked` _aswbp_dialog_option))

(event `Key|Enter`
  (params (Key :type "Key Structure"))
  (:`Pressed`
    (goto _label)))

(event `self.Second.OnClicked`
  (params (TouchedComponent :type "PrimitiveComponent Object Reference") (ButtonPressed :type "Key Structure"))
  ;[1 1 1] OnButtonClick
  (bind _aswbp_dialog_option (cast `/Game/PathOfDestruction/UI/WBP_DialogOption` (`WidgetComponent.GetWidget` (`self.Second`))))
  (`/Game/PathOfDestruction/UI/WBP_DialogOption.Clicked` _aswbp_dialog_option))

(event `self.ReceivePossessed`
  (params (NewController :type "Controller Object Reference"))
  (bind _returnvalue (`GameplayStatics.GetPlayerController` 0))
  (bind _hud (`/Game/PathOfDestruction/Core/BP_PlayerController.HUD` (cast `/Game/PathOfDestruction/Core/BP_PlayerController` (`GameplayStatics.GetPlayerController` 0) :!pure true)))
  ;[1 1 1] On (un)possessed
  (`/Engine/EditorBlueprintResources/StandardMacros.IsValid` _returnvalue
    (:`Is Valid`
      (set `PlayerController.bShowMouseCursor` true _returnvalue)
      (`WidgetBlueprintLibrary.SetInputMode_GameAndUIEx` _returnvalue (`WidgetComponent.GetWidget` (`self.First`)) "LockAlways" false)
      (`self.Update` (`self.DlgContext`))
      (`self.SetActorTickEnabled` true)
      (`/Engine/EditorBlueprintResources/StandardMacros.IsValid` _hud
        (:`Is Valid`
          (`UserWidget.PlayAnimation` _hud (`/Game/PathOfDestruction/UI/WBP_Menu.Open` _hud) 0.0 1 "Forward" 1.0 false)
          (`KismetSystemLibrary.Delay` 1.0))))))

(event `self.ReceiveBeginPlay`
  ;[1 1 1] BeginPlay
  (bind _aswbp_dialog_option (cast `/Game/PathOfDestruction/UI/WBP_DialogOption` (`WidgetComponent.GetWidget` (`self.Second`))))
  (set `/Game/PathOfDestruction/UI/WBP_DialogOption.OptionIndex` 1 _aswbp_dialog_option))

(event `self.ReceiveUnpossessed`
  (params (OldController :type "Controller Object Reference"))
  (bind _returnvalue (`GameplayStatics.GetPlayerController` 0))
  ;[1 1 1] On (un)possessed
  (`/Engine/EditorBlueprintResources/StandardMacros.IsValid` _returnvalue
    (:`Is Valid`
      (set `PlayerController.bShowMouseCursor` false _returnvalue))))

(event `SetDisType`
  (params (DisType :type Name))
  (bind _hud (`/Game/PathOfDestruction/Core/BP_PlayerController.HUD` (cast `/Game/PathOfDestruction/Core/BP_PlayerController` (`GameplayStatics.GetPlayerController` 0) :!pure true)))
  ;[1 1 1] Set dialog's disadvantages
  (`SceneComponent.K2_SetRelativeLocation` (`self.Second`) (0.0 0.0 -100.0) false true)
  (`SceneComponent.K2_SetRelativeLocation` (`self.First`) (0.0 0.0 100.0) false true)
  (bind _outactors (`GameplayStatics.GetAllActorsOfClass` "/Game/PathOfDestruction/DialogScreen/BP_Button.BP_Button_C"))
  (for _array_element _outactors
    (`self.K2_DestroyActor` _array_element))
  (`self.Stop`)
  (switch `name` DisType
    (:`None`
      (set `self.TypeOfDisadvantage` "NewEnumerator1")
      (`/Engine/EditorBlueprintResources/StandardMacros.IsValid` _hud
        (:`Is Valid`
          (`UserWidget.StopAnimation` _hud (`/Game/PathOfDestruction/UI/WBP_Menu.RunText` _hud)))
        (:`Is Not Valid`
          _))
      (if (not (`DlgContext.IsValidOptionIndex` (`self.DlgContext`) 1))
        (`SceneComponent.K2_SetRelativeLocation` (`self.Second`) (-1000.0 -1000.0 -1000.0) false true)
        (`SceneComponent.K2_SetRelativeLocation` (`self.First`) (-1000.0 -1000.0 -1000.0) false true)))
    (:`BouncingButton`
      (set `self.TypeOfDisadvantage` "NewEnumerator0"))
    (:`LotsOfButtons`
      (set `self.TypeOfDisadvantage` "NewEnumerator2"))))

(event `Update`
  (params (Context :type "DlgContext Object Reference"))
  ;[1 1 1] Update
  (`/Engine/EditorBlueprintResources/StandardMacros.IsValid` Context
    (:`Is Valid`
      (`|ExecutionSequence`
        (:`then_0`
          ;;[1 1 1] 1. Set name and text
          (bind _aswbp_dialog_widget (cast `/Game/PathOfDestruction/UI/WBP_DIalogWidget` (`WidgetComponent.GetWidget` (`self.DialogBox`))))
          (`TextBlock.SetText` (`/Game/PathOfDestruction/UI/WBP_DIalogWidget.Name` _aswbp_dialog_widget) (`DlgContext.GetActiveNodeParticipantDisplayName` Context))
          (`MultiLineEditableTextBox.SetText` (`/Game/PathOfDestruction/UI/WBP_DIalogWidget.Text` _aswbp_dialog_widget) (`DlgContext.GetActiveNodeText` Context)))
        (:`then_1`
          ;;[1 1 1] 2. Add options
          (bind _aswbp_dialog_option (cast `/Game/PathOfDestruction/UI/WBP_DialogOption` (`WidgetComponent.GetWidget` (`self.First`))))
          (`/Game/PathOfDestruction/UI/WBP_DialogOption.Update` _aswbp_dialog_option Context)
          (bind _aswbp_dialog_option_2 (cast `/Game/PathOfDestruction/UI/WBP_DialogOption` (`WidgetComponent.GetWidget` (`self.Second`))))
          (`/Game/PathOfDestruction/UI/WBP_DialogOption.Update` _aswbp_dialog_option_2 Context)
          (`self.RefreshButtons`))))
    (:`Is Not Valid`
      (`self.DialogEnd`))))

(event `DialogEnd`
  (bind _hud (`/Game/PathOfDestruction/Core/BP_PlayerController.HUD` (cast `/Game/PathOfDestruction/Core/BP_PlayerController` (`GameplayStatics.GetPlayerController` 0) :!pure true)))
  (bind _hud_2 (`/Game/PathOfDestruction/Core/BP_PlayerController.HUD` (cast `/Game/PathOfDestruction/Core/BP_PlayerController` (`GameplayStatics.GetPlayerController` 0) :!pure true)))
  ;[1 1 1] DialogEnd
  (`SceneComponent.K2_SetRelativeLocation` (`self.Second`) (-1000.0 -1000.0 -1000.0) false true)
  (`SceneComponent.K2_SetRelativeLocation` (`self.First`) (-1000.0 -1000.0 -1000.0) false true)
  (bind _returnvalue (`GameplayStatics.GetActorOfClass` "/Game/PathOfDestruction/Core/BP_Char.BP_Char_C"))
  (`UserWidget.PlayAnimation` _hud_2 (`/Game/PathOfDestruction/UI/WBP_Menu.Close` _hud_2) 0.0 1 "Forward" 1.0 false)
  (`KismetSystemLibrary.Delay` 1.0)
  (`Controller.Possess` (`GameplayStatics.GetPlayerController` 0) _returnvalue)
  (`self.SetActorTickEnabled` false)
  (`WidgetBlueprintLibrary.SetInputMode_GameOnly` (`GameplayStatics.GetPlayerController` 0))
  (`UserWidget.PlayAnimation` _hud (`/Game/PathOfDestruction/UI/WBP_Menu.Open` _hud) 0.0 1 "Forward" 1.0 false)
  (`KismetSystemLibrary.Delay` 1.0))

(event `self.ReceiveTick`
  (params (DeltaSeconds :type "Float (single-precision)"))
  (bind _hud (`/Game/PathOfDestruction/Core/BP_PlayerController.HUD` (cast `/Game/PathOfDestruction/Core/BP_PlayerController` (`GameplayStatics.GetPlayerController` 0) :!pure true)))
  (bind _aswbp_dialog_option (cast `/Game/PathOfDestruction/UI/WBP_DialogOption` (select `bool` (`self.LeftDefected`) :`false` (`WidgetComponent.GetWidget` (`self.Second`)) :`true` (`WidgetComponent.GetWidget` (`self.First`))) :!pure true))
  (switch `/Game/PathOfDestruction/Core/E_DisadvantageType` (`self.TypeOfDisadvantage`)
    (:`NewEnumerator0`
      (`/Engine/EditorBlueprintResources/StandardMacros.DoOnce` false :!label _label_2
        (:`Completed`
          (`KismetSystemLibrary.MoveComponentTo` (select `bool` (`self.LeftDefected`) :`false` (`self.Second`) :`true` (`self.First`) :!type "SceneComponent Object Reference") (`KismetMathLibrary.MakeVector` (`KismetMathLibrary.RandomFloatInRange` -570.0 570.0) 0.0 (`KismetMathLibrary.RandomFloatInRange` -430.0 430.0)) (struct :`Yaw` 90.0) false false 0.5 :!label _label_3)
          (goto _label_2 :!via `Reset`))))
    (:`NewEnumerator2`
      (`/Engine/EditorBlueprintResources/StandardMacros.DoOnce` true :!label _label_4
        (:`Completed`
          (`|ExecutionSequence`
            (:`then_0`
              (bind _output_get (set `self.RandomSeed` (`KismetMathLibrary.RandomIntegerInRange` 0 27))))
            (:`then_1`
              (for _index (range 28)
                (if (== _output_get _index)
                  (bind _output (`|GetArrayItem` (`self.PossitionArray`) _index))
                  (`SceneComponent.K2_SetRelativeLocation` (select `bool` (`self.LeftDefected`) :`false` (`self.First`) :`true` (`self.Second`) :!type "SceneComponent Object Reference") _output false true)
                  (else
                    (bind _returnvalue (`|SpawnActorFromClass` "/Game/PathOfDestruction/DialogScreen/BP_Button.BP_Button_C" (`KismetMathLibrary.MakeTransform` _output (struct :`Yaw` 90.0)) "Undefined" "OverrideRootScale" null null))
                    (`self.K2_AttachToActor` _returnvalue self "DefaultSceneRoot" "KeepRelative" "KeepRelative" "KeepRelative" true)
                    (bind _returnvalue_2 (`/Game/PathOfDestruction/UI/WBP_DialogOption.F_GetText` _aswbp_dialog_option))
                    (bind _aswbp_dialog_option_2 (cast `/Game/PathOfDestruction/UI/WBP_DialogOption` (`WidgetComponent.GetWidget` (`/Game/PathOfDestruction/DialogScreen/BP_Button.ButtonWidget` _returnvalue)) :!pure true))
                    (`TextBlock.SetText` (`/Game/PathOfDestruction/UI/WBP_DialogOption.OptionText` _aswbp_dialog_option_2) _returnvalue_2)
                    (set `/Game/PathOfDestruction/UI/WBP_DialogOption.OptionIndex` (`/Game/PathOfDestruction/UI/WBP_DialogOption.OptionIndex` _aswbp_dialog_option) _aswbp_dialog_option_2))))
              (`SceneComponent.K2_SetRelativeLocation` (select `bool` (`self.LeftDefected`) :`false` (`self.Second`) :`true` (`self.First`)) (-1000.0 -1000.0 -1000.0) false true))
            (:`then_2`
              (`UserWidget.PlayAnimation` _hud (`/Game/PathOfDestruction/UI/WBP_Menu.RunText` _hud) 0.0 0 "Forward" 1.0 false))))))))

(event `Stop`
  (`|ExecutionSequence`
    (:`then_0`
      (`self.RefreshButtons`))
    (:`then_1`
      (goto _label_3 :!via `Stop`))))

(event `RefreshButtons`
  (goto _label_4 :!via `Reset`))

(fn `UserConstructionScript`)
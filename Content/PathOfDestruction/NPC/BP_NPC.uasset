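; BP_NPC is an NPC actor that starts a dialogue when the player character enters its trigger box.
; On overlap it plays the HUD's Close animation, waits a second, disables further overlap events, then calls DialogStart on BP_Char with its Dialog and itself.
; It implements dialogue participant functions, supplying name and display name, while conditions, values and events are stubs returning defaults.
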(event `self.Box.OnComponentBeginOverlap`
  (params (OverlappedComponent :type "PrimitiveComponent Object Reference") (OtherActor :type "Actor Object Reference") (OtherComp :type "PrimitiveComponent Object Reference") (OtherBodyIndex :type Integer) (bFromSweep :type Boolean) (SweepResult :type "HitResult Structure (by ref)"))
  (bind _hud (`/Game/PathOfDestruction/Core/BP_PlayerController.HUD` (cast `/Game/PathOfDestruction/Core/BP_PlayerController` (`GameplayStatics.GetPlayerController` 0) :!pure true)))
  (bind _asbp_char (cast `/Game/PathOfDestruction/Core/BP_Char` OtherActor))
  (`UserWidget.PlayAnimation` _hud (`/Game/PathOfDestruction/UI/WBP_Menu.Close` _hud) 0.0 1 "Forward" 1.0 false)
  (`KismetSystemLibrary.Delay` 1.0)
  (set `PrimitiveComponent.bGenerateOverlapEvents` false (`self.Box`))
  (`/Game/PathOfDestruction/Core/BP_Char.DialogStart` _asbp_char (`self.Dialog`) self))

(fn `CheckCondition`
  (params (Context :type "DlgContext Object Reference") (ConditionName :type Name))
  (returns (ReturnValue :type Boolean))
  (return false))

(fn `GetBoolValue`
  (params (ValueName :type Name))
  (returns (ReturnValue :type Boolean))
  (return false))

(fn `GetFloatValue`
  (params (ValueName :type Name))
  (returns (ReturnValue :type "Float (double-precision)"))
  (return 0.0))

(fn `GetIntValue`
  (params (ValueName :type Name))
  (returns (ReturnValue :type Integer))
  (return 0))

(fn `GetNameValue`
  (params (ValueName :type Name))
  (returns (ReturnValue :type Name))
  (return "None"))

(fn `GetParticipantDisplayName`
  (params (ActiveSpeaker :type Name))
  (returns (ReturnValue :type Text))
  (return (`self.DialogueParticipantDisplayName `)))

(fn `GetParticipantGender`
  (returns (ReturnValue :type "ETextGender Enum"))
  (return "Masculine"))

(fn `GetParticipantIcon`
  (params (ActiveSpeaker :type Name) (ActiveSpeakerState :type Name))
  (returns (ReturnValue :type "Texture2D Object Reference"))
  (return null))

(fn `GetParticipantName`
  (returns (ReturnValue :type Name))
  (return (`self.ParticipantName`)))

(fn `ModifyBoolValue`
  (params (ValueName :type Name) (bNewValue :type Boolean))
  (returns (ReturnValue :type Boolean))
  (return false))

(fn `ModifyFloatValue`
  (params (ValueName :type Name) (bDelta :type Boolean) (Value :type "Float (double-precision)"))
  (returns (ReturnValue :type Boolean))
  (return false))

(fn `ModifyIntValue`
  (params (ValueName :type Name) (bDelta :type Boolean) (Value :type Integer))
  (returns (ReturnValue :type Boolean))
  (return false))

(fn `ModifyNameValue`
  (params (ValueName :type Name) (NameValue :type Name))
  (returns (ReturnValue :type Boolean))
  (return false))

(fn `OnDialogueEvent`
  (params (Context :type "DlgContext Object Reference") (EventName :type Name))
  (returns (ReturnValue :type Boolean))
  (return false))

(fn `UserConstructionScript`)